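; BP_Test is a test actor that moves its Sphere component continuously and prints a greeting on BeginPlay.
; Each Tick offsets the Sphere's world location by Speed scaled by delta time, keeping rotation and scale, with no sweep.
; A Kill event resets the actor's transform to the world origin with zero rotation and unit scale rather than destroying it.
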(event `self.ReceiveBeginPlay`
  (`KismetSystemLibrary.PrintString` "Hello"))

(event `self.ReceiveTick`
  (params (DeltaSeconds :type "Float (single-precision)"))
  (`SceneComponent.K2_SetWorldTransform` (`self.Sphere`) (`KismetMathLibrary.MakeTransform` (+ (.location (`SceneComponent.K2_GetComponentToWorld` (`self.Sphere`))) (* DeltaSeconds (`self.Speed`))) (.rotation (`SceneComponent.K2_GetComponentToWorld` (`self.Sphere`))) (.scale (`SceneComponent.K2_GetComponentToWorld` (`self.Sphere`)))) false false))

(event `Kill`
  (`self.K2_SetActorTransform` (`KismetMathLibrary.MakeTransform` (0.0 0.0 0.0))))

(fn `UserConstructionScript`)